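; BP_ActorTest is a test actor that assigns itself a Name from four hardcoded adjectives in its Construction Script.
; It intends a random pick via Shuffle and index zero, but the literal array appears rebuilt for the read, likely always yielding "Wailing".
; The branch is hardwired true, leaving the empty-Name check unused, so Name is overwritten on every construction.
; The event graph holds only disabled placeholder events.
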(fn `UserConstructionScript`
  (bind _array (`|MakeArray` "Wailing" "Peerless" "Desolute" "Isloated"))
  (if true
    (`KismetArrayLibrary.Array_Shuffle` _array)
    (set `self.Name` (`|GetArrayItem` _array))))