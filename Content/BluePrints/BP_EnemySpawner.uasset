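; BP_EnemySpawner keeps the level stocked with enemies, spawning a new wave whenever none remain.
; On BeginPlay it gathers all BP_EnemySpawnLocation actors, prints their count and spawns BP_Enemy at each with an 80% chance.
; A self-calling EnemyCountCheck event waits two seconds while any enemy exists, otherwise spawns again and rechecks immediately, avoiding Tick.
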(event `EnemyCountCheck`
  (bind _outactors (`GameplayStatics.GetAllActorsOfClass` "/Game/BluePrints/BP_Enemy.BP_Enemy_C"))
  (if (> (`KismetArrayLibrary.Array_Length` _outactors) 0)
    (`KismetSystemLibrary.Delay` 2.0)
    (else
      (`self.SpawnEnemies`)))
  (`self.EnemyCountCheck`) ; loop this forevver
)

(event `self.ReceiveBeginPlay`
  (bind _outactors (`GameplayStatics.GetAllActorsOfClass` "/Game/BluePrints/BP_EnemySpawnLocation.BP_EnemySpawnLocation_C"))
  (`KismetSystemLibrary.PrintString` (`KismetStringLibrary.Concat_StrStr` "There are" (`KismetStringLibrary.Conv_IntToString` (`KismetArrayLibrary.Array_Length` _outactors)) "spawners in the level") true true (struct :`G` 0.66 :`B` 1.0 :`A` 1.0) 10.0)
  (`self.SpawnEnemies`)
  (`self.EnemyCountCheck`))

(event `SpawnEnemies`
  (for _array_element (stale `self.ReceiveBeginPlay` _outactors)
    (if (< (`KismetMathLibrary.RandomFloat`) 0.8)
      (`|SpawnActorFromClass` "/Game/BluePrints/BP_Enemy.BP_Enemy_C" (`self.GetTransform` _array_element) "Undefined" "MultiplyWithRoot" null null))))

(fn `UserConstructionScript`)