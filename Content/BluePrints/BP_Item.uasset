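; BP_Item is an item Blueprint with a name, damage value and elemental type, which prints debug info on BeginPlay.
; BeginPlay calls an empty Construnctor function, then prints the name, element and GetDamage result against a test victim element labelled air.
; GetDamage matches the opposing element using a +2 modulo 4 wrap on the enum.
; A match currently still returns base Damage, as the doubling node is unused.
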(event `self.ReceiveBeginPlay`
  (`self.Construnctor`)
  (`KismetSystemLibrary.PrintString` (`KismetStringLibrary.Concat_StrStr` (`self.name`)))
  (bind _damage (`self.GetDamage` "NewEnumerator0"))
  (`KismetSystemLibrary.PrintString` (`KismetStringLibrary.Concat_StrStr` "our elem type is " (`|GetEnumeratorNameAsString` (`self.ElementalType`)) ", vitcim is air, damage=" (`KismetStringLibrary.Conv_IntToString` _damage)) true true (struct :`R` 0.527778 :`B` 0.01702 :`A` 1.0) 5.0))

(fn `Construnctor`)

(fn `GetDamage`
  (params (`Victim ElementalType` :type "/Game/BluePrints/ElementalType Enum" :default "NewEnumerator0"))
  (returns (Damage :type Integer))
  (locals (`Return Damage` :type Integer :default 0) (NewLocalVar_0 :type Integer :default 0))
  (set `local.Return Damage` (`self.Damage`))
  (if (== (mod (+ `Victim ElementalType` 2) 4) (`KismetMathLibrary.Conv_ByteToInt` (`self.ElementalType`)))
    (set `local.Return Damage` (`self.Damage`)) ; set return dmg to this items dmg
  )
  (return (`local.Return Damage`)))

(fn `UserConstructionScript`)