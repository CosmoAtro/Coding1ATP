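; BP_CoolBox is a spawner actor that endlessly produces BP_Key actors above its Cube component.
; On BeginPlay it computes a spawn point at a fixed height over the cube and prints debug messages with its name and that location.
; It then spawns a randomly scaled key and loops back through a Delay set by SpawnDelay, with no stop condition.
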(event `self.ReceiveBeginPlay`
  (set `self.KeySpawnLocation` (+ (`SceneComponent.K2_GetComponentLocation` (`self.Cube`)) (0.0 0.0 200.0)))
  (`KismetSystemLibrary.PrintString` (`KismetStringLibrary.Concat_StrStr` (`KismetSystemLibrary.GetDisplayName` self) " I exist! I am suffering") true true (struct :`G` 0.66 :`B` 1.0 :`A` 1.0) 10.0) ; Just like cout
  (`KismetSystemLibrary.PrintString` (`KismetStringLibrary.Conv_VectorToString` (`self.KeySpawnLocation`)) true true (struct :`R` 0.621257 :`G` 0.630753 :`B` 1.0 :`A` 1.0) 10.0)
  (`KismetSystemLibrary.PrintString` (`KismetStringLibrary.Conv_VectorToString` (`self.KeySpawnLocation`)) true true (struct :`R` 0.041643 :`B` 1.0 :`A` 1.0) 10.0)
  (`|SpawnActorFromClass` "/Game/BluePrints/BP_Key.BP_Key_C" (`KismetMathLibrary.MakeTransform` (`self.KeySpawnLocation`) (struct) (* 1.0 (`KismetMathLibrary.RandomFloatInRange` 0.1 2.0))) "Undefined" "MultiplyWithRoot" null null :!label _label)
  (`KismetSystemLibrary.Delay` (`self.Spawn Delay`))
  (goto _label))

(fn `UserConstructionScript`)